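; StefanoCharacter is a playable character Blueprint handling basic movement and jumping through Enhanced Input.
; On BeginPlay it adds the SteInputMap mapping context to the local player's Enhanced Input subsystem.
; MoveInput drives movement along the control rotation's yaw and roll with pitch zeroed, and tracks an IsHoldingMove flag on start and completion.
; JumpInput starts and stops jumping.
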(event `self.ReceiveBeginPlay`
  ;[0.3375 1 0.1599] Movement
  (bind _asplayer_controller (cast `PlayerController` (`self.GetController`)))
  (bind _returnvalue (pcsubsystem `EnhancedInputLocalPlayerSubsystem` _asplayer_controller))
  (`/Engine/EditorBlueprintResources/StandardMacros.IsValid` _returnvalue
    (:`Is Valid`
      (message `EnhancedInputSubsystemInterface.AddMappingContext` _returnvalue "/Game/Insomnia/Input/SteInputMap.SteInputMap" 0 (struct)))))

(event `EnhancedInput|/Game/Insomnia/Input/MoveInput`
  (params (ActionValue :type "Vector2D Structure") (ElapsedSeconds :type "Float (double-precision)") (TriggeredSeconds :type "Float (double-precision)") (InputAction :type "InputAction Object Reference" :default "/Game/Insomnia/Input/MoveInput.MoveInput"))
  (bind (_returnvalue_roll _returnvalue_pitch _returnvalue_yaw) (`KismetMathLibrary.BreakRotator` (`self.GetControlRotation`)))
  (bind (_returnvalue_roll_2 _returnvalue_pitch_2 _returnvalue_yaw_2) (`KismetMathLibrary.BreakRotator` (`self.GetControlRotation`)))
  ;[0.3375 1 0.1599] Movement
  (:`Triggered`
    (`self.AddMovementInput` (`KismetMathLibrary.GetRightVector` (`KismetMathLibrary.MakeRotator` _returnvalue_roll 0.0 _returnvalue_yaw)) ActionValue_X)
    (`self.AddMovementInput` (`KismetMathLibrary.GetForwardVector` (`KismetMathLibrary.MakeRotator` _returnvalue_roll_2 0.0 _returnvalue_yaw_2)) ActionValue_Y))
  (:`Started`
    (set `self.isHoldingMove` true))
  (:`Completed`
    (set `self.isHoldingMove` false)))

(event `EnhancedInput|/Game/Insomnia/Input/JumpInput`
  (params (ActionValue :type Boolean) (ElapsedSeconds :type "Float (double-precision)") (TriggeredSeconds :type "Float (double-precision)") (InputAction :type "InputAction Object Reference" :default "/Game/Insomnia/Input/JumpInput.JumpInput"))
  (:`Triggered`
    (`self.Jump`))
  (:`Completed`
    (`self.StopJumping`)))

(fn `UserConstructionScript`)