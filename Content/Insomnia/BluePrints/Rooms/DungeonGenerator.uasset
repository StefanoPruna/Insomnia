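; DungeonGenerator is an actor that starts building a room-based dungeon on BeginPlay.
; It spawns a RoomOne start room at its own root transform and gathers that room's Exits children into ExitsList.
; It then spawns one random RoomList class at a random exit's transform and stores it as LatestRoom if it is a MasterRoom.
; Generation stops there, with no loop or overlap check.
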(event `self.ReceiveBeginPlay`
  (`self.SpawnStartRoom`)
  (`self.SpawnNextRoom`))

(event `SpawnStartRoom`
  ;[0.05237 1 0.1051] Spawn Start Room
  (bind _returnvalue (`|SpawnActorFromClass` "/Game/Insomnia/BluePrints/Rooms/RoomOne.RoomOne_C" (`SceneComponent.K2_GetComponentToWorld` (`self.DefaultSceneRoot`)) "AlwaysSpawn" "MultiplyWithRoot" null null))
  (`KismetArrayLibrary.Array_Append` (`self.ExitsList`) (`SceneComponent.GetChildrenComponents` (`/Game/Insomnia/BluePrints/Rooms/MasterRoom.Exits` _returnvalue) false)))

(event `SpawnNextRoom`
  (set `self.SelectedExitPoint` (`KismetArrayLibrary.Array_Random` (`self.ExitsList`)))
  (bind _returnvalue (`|SpawnActorFromClass` (`KismetArrayLibrary.Array_Random` (`self.RoomList`)) (`SceneComponent.K2_GetComponentToWorld` (`self.SelectedExitPoint`)) "AlwaysSpawn" "MultiplyWithRoot" null null))
  (bind _asmaster_room (cast `/Game/Insomnia/BluePrints/Rooms/MasterRoom` _returnvalue))
  (set `self.LatestRoom` _asmaster_room) ; Latest room that has been spawned
)

(fn `UserConstructionScript`)